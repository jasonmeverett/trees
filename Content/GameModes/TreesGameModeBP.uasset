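; Game mode for a tree scene that lets the player remove trees with the mouse and quit with Escape.
; On BeginPlay it turns on the stat unit display and enables input on itself, so the game mode handles key events directly.
; Right-click traces complex collision under the cursor on the Visibility channel, prints the hit actor's name and destroys it if its class derives from BasicTree.
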(event EventBeginPlay
  (Development|ExecuteConsoleCommand "stat unit" 0)
  (Input|EnableInput (Game|GetPlayerController 0)))

(event EventTick
  (params (DeltaSeconds :type Float%20%28single-precision%29)))

(event Input|KeyboardEvents|Escape
  (params (Key :type Key%20Structure :default "None"))
  (:Pressed
    (Game|QuitGame 0 "Quit" false)))

(event Input|MouseEvents|RightMouseButton
  (params (Key :type Key%20Structure :default "None"))
  (bind _returnvalue (Game|GetPlayerController 0))
  (bind _hitresult (Game|Player|GetHitResultUnderCursorbyChannel _returnvalue "TraceTypeQuery1" true))
  (bind _hitactor (Collision|BreakHitResult _hitresult))
  (:Pressed
    (Development|PrintString (Utilities|GetDisplayName _hitactor))
    (if (Utilities|ClassIsChildOf (Utilities|GetClass _hitactor) "/Game/Trees/BasicTree.BasicTree_C")
      (Actor|DestroyActor _hitactor))))

(fn ConstructionScript)